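; Minecraft-style voxel terrain actor that generates block ground and lets the player place blocks.
; The construction script fills a grid with Grass instances, setting height from two summed sine-product waves, and stacks Dirt instances beneath at fixed 100-unit steps.
; Number keys pick a block type; left click traces from the first-person camera and adds that instance at the grid-snapped impact point, without checking for a hit.
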(event `self.ReceiveBeginPlay`
  (`self.EnableInput` (`GameplayStatics.GetPlayerController` 0)))

(event `Key|LeftMouseButton`
  (params (Key :type "Key Structure"))
  (bind _grass (`self.Grass`))
  (bind _returnvalue (`KismetMathLibrary.Conv_IntToDouble` (`self.Tile Size`)))
  (:`Pressed`
    (`KismetSystemLibrary.PrintString` "pew pew")
    (bind _asfirst_person_character (cast `/Game/FirstPersonBP/Blueprints/FirstPersonCharacter` (`GameplayStatics.GetPlayerCharacter` 0)))
    (bind _firstpersoncamera (`/Game/FirstPersonBP/Blueprints/FirstPersonCharacter.FirstPersonCamera` _asfirst_person_character))
    (bind _returnvalue_2 (`SceneComponent.K2_GetComponentLocation` _firstpersoncamera))
    (bind _outhit (`KismetSystemLibrary.LineTraceSingle` :`Start` _returnvalue_2 :`End` (+ _returnvalue_2 (* (`SceneComponent.GetForwardVector` _firstpersoncamera) 1000.0)) :`TraceChannel` "TraceTypeQuery1" :`bIgnoreSelf` false))
    (`InstancedStaticMeshComponent.AddInstance` (select `int` (`self.Block Type`) :`0` _grass :`1` _grass :`2` (`self.Dirt`) :`3` (`self.Stone`) :`4` (`self.Diamond Ore`) :`5` (`self.Diamond Block`)) (`KismetMathLibrary.MakeTransform` (`KismetMathLibrary.MakeVector` (`KismetMathLibrary.GridSnap_Float` (.x (`.ImpactPoint` (`GameplayStatics.BreakHitResult` _outhit))) _returnvalue) (`KismetMathLibrary.GridSnap_Float` (.y (`.ImpactPoint` (`GameplayStatics.BreakHitResult` _outhit))) _returnvalue) (`KismetMathLibrary.GridSnap_Float` (.z (`.ImpactPoint` (`GameplayStatics.BreakHitResult` _outhit))) _returnvalue))) false)))

(event `Key|One`
  (params (Key :type "Key Structure"))
  (:`Pressed`
    (bind _output_get (set `self.Block Type` 1))
    (`KismetSystemLibrary.PrintString` (`KismetStringLibrary.Conv_IntToString` _output_get))))

(event `Key|Two`
  (params (Key :type "Key Structure"))
  (:`Pressed`
    (bind _output_get (set `self.Block Type` 2))
    (`KismetSystemLibrary.PrintString` (`KismetStringLibrary.Conv_IntToString` _output_get))))

(event `Key|Three`
  (params (Key :type "Key Structure"))
  (:`Pressed`
    (bind _output_get (set `self.Block Type` 3))
    (`KismetSystemLibrary.PrintString` (`KismetStringLibrary.Conv_IntToString` _output_get))))

(event `Key|Four`
  (params (Key :type "Key Structure"))
  (:`Pressed`
    (bind _output_get (set `self.Block Type` 4))
    (`KismetSystemLibrary.PrintString` (`KismetStringLibrary.Conv_IntToString` _output_get))))

(event `Key|Five`
  (params (Key :type "Key Structure"))
  (:`Pressed`
    (bind _output_get (set `self.Block Type` 5))
    (`KismetSystemLibrary.PrintString` (`KismetStringLibrary.Conv_IntToString` _output_get))))

(fn `UserConstructionScript`
  (bind _tile_size (`self.Tile Size`))
  (bind _tile_size_2 (`self.Tile Size`))
  (bind _length (`self.Length`))
  (bind _width (`self.Width`))
  (bind _terrain_wave_frequency (`self.Terrain Wave Frequency`))
  (bind _terrain_wave_frequency_2 (`self.Terrain Wave Frequency`))
  ;[1 1 1] Iterate Through Each Coordinate; Range:
  ; -length <= x <= length
  ; -width <= y <= width
  (for _index (range (* _length -1) (+ _length 1))
    (for _index_2 (range (* _width -1) (+ _width 1))
      (bind _returnvalue (`KismetMathLibrary.Conv_IntToDouble` (* _index _tile_size)))
      (bind _returnvalue_2 (`KismetMathLibrary.Conv_IntToDouble` (* _index_2 _tile_size)))
      (bind _returnvalue_3 (`KismetMathLibrary.Conv_IntToDouble` (+ (* (`KismetMathLibrary.Round` (* (`KismetMathLibrary.DegSin` (* (* _index _terrain_wave_frequency_2) 1.4)) (`KismetMathLibrary.DegSin` (* (* _index_2 _terrain_wave_frequency_2) 0.8)) (`self.Height Variation`))) _tile_size_2) (* (`KismetMathLibrary.Round` (* (`KismetMathLibrary.DegSin` (* (* _index _terrain_wave_frequency) 0.7)) (`KismetMathLibrary.DegSin` (* (* _index_2 _terrain_wave_frequency) 0.9)) (`self.Height Variation`))) _tile_size_2))))
      (bind _returnvalue_4 (`KismetMathLibrary.MakeVector` _returnvalue _returnvalue_2 _returnvalue_3))
      ;[1 1 1] Create Block at Coordinate
      (`InstancedStaticMeshComponent.AddInstance` (`self.Grass`) (`KismetMathLibrary.Conv_VectorToTransform` _returnvalue_4) false)
      ;;[1 1 1] debug
      (`KismetSystemLibrary.PrintString` (`KismetStringLibrary.Conv_VectorToString` _returnvalue_4))
      ;[1 1 1] Make {x} More Levels of Dirt Blocks to Go Beneath Each Intance of Grass Blocks at Each Coordinate
      (for _index_3 (range 1 (+ (`self.Block Depth`) 1))
        (`InstancedStaticMeshComponent.AddInstance` (`self.Dirt`) (`KismetMathLibrary.Conv_VectorToTransform` (`KismetMathLibrary.MakeVector` _returnvalue _returnvalue_2 (- _returnvalue_3 (* _index_3 100.0)))) false)))))